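; BP_Door is a door actor that slides away from its starting position at dusk and back at dawn.
; On BeginPlay it waits a tick, stores its location, then binds to the dawn and dusk events of the BP_DayTimeManager found in the level.
; A MoveActor timeline plays at dusk and reverses at dawn, adding its vector track to the stored location without sweeping.
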(event Custom|OnDawnEvent
  (bind _newtrack_1 (Timeline|MoveActor Reverse)
    (:Update
      (Transformation|SetActorLocation (+ (Variables|Default|GetStartLocation) _newtrack_1) false false))))

(event Custom|OnDuskEvent
  (bind _newtrack_1 (Timeline|MoveActor Play)
    (:Update
      (Transformation|SetActorLocation (+ (Variables|Default|GetStartLocation) _newtrack_1) false false))))

(event EventBeginPlay
  (Utilities|FlowControl|DelayUntilNextTick)
  (Utilities|FlowControl|Sequence
    (:then_0
      (Variables|Default|SetStartLocation (Transformation|GetActorLocation)))
    (:then_1
      (bind _returnvalue (Actor|GetActorOfClass "/Game/Blueprints/BP_DayTimeManager.BP_DayTimeManager_C"))
      (Utilities|IsValid _returnvalue
        (:Is%20Valid
          (EventDispatchers|BindEventtoOnDawn _returnvalue (EventDispatchers|CreateEvent :!event Custom|OnDawnEvent))
          (EventDispatchers|BindEventtoOnDusk _returnvalue (EventDispatchers|CreateEvent :!event Custom|OnDuskEvent)))))))

(event Collision|EventActorBeginOverlap
  (params (OtherActor :type Actor%20Object%20Reference)))

(event EventTick
  (params (DeltaSeconds :type Float%20%28single-precision%29)))

(fn ConstructionScript)