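; Actor component that computes a diminishing-returns multiplier that shrinks with each counted use.
; On BeginPlay it binds an event to OnUsed on the owner's BPC_EmitterComponent; its HandleUse event has no logic.
; CalculateDiminishingReturnValue subtracts a linear percentage loss from the base multiplier, clamps it to a minimum and increments the use count.
; It returns zero once the count equals MaxUses.
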(event Custom|HandleUse
  (params (Instigator :type Actor%20Object%20Reference) (UsedActor :type Actor%20Object%20Reference)))

(event EventBeginPlay
  (EventDispatchers|BindEventtoOnUsed (Actor|GetComponentbyClass (Components|GetOwner) "/Game/Blueprints/BPC_EmitterComponent.BPC_EmitterComponent_C") (EventDispatchers|CreateEvent :!event Custom|HandleUse)))

(event EventTick
  (params (DeltaSeconds :type Float%20%28single-precision%29)))

(fn CalculateDiminishingReturnValue
  (if (== (Variables|Default|GetMaxUses) (Variables|Default|GetCurrentUses))
    (return 0.0)
    (else
      (LocalVariables|SetLocalLossPerUse (/ (Variables|Default|GetPercentLossPerUse) 1e+02))
      (LocalVariables|SetLocalTotalLoss (* (LocalVariables|GetLocalLossPerUse) (Variables|Default|GetCurrentUses)))
      (LocalVariables|SetLocalMultiplier (- (Variables|Default|GetBaseMultiplier) (LocalVariables|GetLocalTotalLoss)))
      (if (< (LocalVariables|GetLocalMultiplier) (Variables|Default|GetMinMultiplier))
        (bind _output_get (LocalVariables|SetLocalMultiplier (Variables|Default|GetMinMultiplier)))
        (Math|Integer|IncrementInt (Variables|Default|GetCurrentUses)
          (:%20%20
            (return _output_get)))
        (else
          (Math|Integer|IncrementInt (Variables|Default|GetCurrentUses)
            (:%20%20
              (return (LocalVariables|GetLocalMultiplier)))))))))