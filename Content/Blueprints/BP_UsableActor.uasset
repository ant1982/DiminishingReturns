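; BP_UsableActor is an interactable actor with a heal amount that diminishes with use, shown on its health widget.
; On BeginPlay it caches its emitter component and initializes the widget with HealAmount.
; Interact, if the emitter is valid, emits a used event, then multiplies the stored HealAmount by the diminishing-returns component's value, so changes compound, and updates the widget.
; It applies no healing itself.
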(event EventBeginPlay
  (bind _returnvalue (Actor|GetComponentbyClass "/Game/Blueprints/BPC_EmitterComponent.BPC_EmitterComponent_C"))
  (Utilities|FlowControl|Sequence
    (:then_0
      (Utilities|IsValid _returnvalue
        (:Is%20Valid
          (Variables|Default|SetEmitterComponent _returnvalue))))
    (:then_1
      (bind _aswbp_health (Utilities|Casting|CastToWBP_Health (UserInterface|GetWidget (Variables|Default|GetWidget))))
      (bind _output_get (Variables|Default|SetAs%20WBP%20Health _aswbp_health))
      (Default|UpdateHealth _output_get (Variables|Default|GetHealAmount)))))

(event Collision|EventActorBeginOverlap
  (params (OtherActor :type Actor%20Object%20Reference)))

(event EventTick
  (params (DeltaSeconds :type Float%20%28single-precision%29)))

(event EventInteract
  (bind _emittercomponent (Variables|Default|GetEmitterComponent))
  (Utilities|IsValid _emittercomponent
    (:Is%20Valid
      (Default|EmitUsed _emittercomponent self)
      (bind _multiplier (Default|CalculateDiminishingReturnValue (Variables|Default|GetBPC_DiminishingReturns)))
      (Variables|Default|SetMultiplier _multiplier)
      (bind _output_get (Variables|Default|SetHealAmount (* (Variables|Default|GetHealAmount) (Variables|Default|GetMultiplier))))
      (Development|PrintString (Utilities|String|ToString(Float) _output_get))
      (Default|UpdateHealth (Variables|Default|GetAs%20WBP%20Health) (Variables|Default|GetHealAmount)))))

(fn ConstructionScript)